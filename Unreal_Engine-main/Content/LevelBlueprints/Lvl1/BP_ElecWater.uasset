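; BP_ElecWater is an electrified water hazard actor that restarts the current level when an unprotected BP_ThirdPersonCharacter touches it.
; Overlapping ZapBox without IsInvincible or IsWaterSafe plays an electricity sound, waits a second, then reopens the level by name.
; Overlapping WhenOff while IsWaterSafe is set destroys the hazard actor.
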(event OnComponentBeginOverlap(zapBox)
  (params (OverlappedComponent :type Primitive%20Component%20Object%20Reference) (OtherActor :type Actor%20Object%20Reference) (OtherComp :type Primitive%20Component%20Object%20Reference) (OtherBodyIndex :type Integer) (bFromSweep :type Boolean) (SweepResult :type Hit%20Result%20Structure%20%28by%20ref%29))
  (bind _asbp_third_person_character (Utilities|Casting|CastToBP_ThirdPersonCharacter OtherActor))
  (if (not (Variables|/Game/ThirdPerson/Blueprints/BP_ThirdPersonCharacter.BP_ThirdPersonCharacter_C|GetisInvincible _asbp_third_person_character))
    (bind _asbp_third_person_character_2 (Utilities|Casting|CastToBP_ThirdPersonCharacter OtherActor))
    (if (not (Variables|/Game/ThirdPerson/Blueprints/BP_ThirdPersonCharacter.BP_ThirdPersonCharacter_C|GetisWaterSafe _asbp_third_person_character_2))
      (Audio|PlaySoundatLocation "/Game/StarterContent/Audio/electricity_us849kj.electricity_us849kj" (Transformation|GetActorLocation) "0, 0, 0" 1.0 1.0 0.0 0 0 0 0)
      (Utilities|FlowControl|Delay 1.0)
      (bind _returnvalue (Game|GetCurrentLevelName true))
      (Game|OpenLevel(byName) (Utilities|String|StringToName _returnvalue)))))

(event OnComponentBeginOverlap(whenOff)
  (params (OverlappedComponent :type Primitive%20Component%20Object%20Reference) (OtherActor :type Actor%20Object%20Reference) (OtherComp :type Primitive%20Component%20Object%20Reference) (OtherBodyIndex :type Integer) (bFromSweep :type Boolean) (SweepResult :type Hit%20Result%20Structure%20%28by%20ref%29))
  (bind _asbp_third_person_character (Utilities|Casting|CastToBP_ThirdPersonCharacter OtherActor))
  (if (Variables|/Game/ThirdPerson/Blueprints/BP_ThirdPersonCharacter.BP_ThirdPersonCharacter_C|GetisWaterSafe _asbp_third_person_character)
    (Actor|DestroyActor)))

(fn ConstructionScript)