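; BP_ElecBox is a Level 1 electrical box that lets the player turn off the electricity when carrying a wrench.
; On overlap it checks the character's HasWrench flag and, if set, calls UpdateIsWaterSafe on that character.
; A DoOnce limits the confirmation text, sound and smoke effect to the first success.
; Without a wrench it prints a warning and plays a failure sound at the world origin.
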(event EventBeginPlay)

(event Collision|EventActorBeginOverlap
  (params (OtherActor :type Actor%20Object%20Reference))
  (bind _returnvalue (Transformation|GetActorLocation))
  (bind _asbp_third_person_character (Utilities|Casting|CastToBP_ThirdPersonCharacter OtherActor))
  (if (Variables|/Game/ThirdPerson/Blueprints/BP_ThirdPersonCharacter.BP_ThirdPersonCharacter_C|GethasWrench _asbp_third_person_character)
    (bind _asbp_third_person_character_2 (Utilities|Casting|CastToBP_ThirdPersonCharacter OtherActor))
    (Default|UpdateIsWaterSafe _asbp_third_person_character_2)
    (Utilities|FlowControl|DoOnce false
      (:Completed
        (Development|PrintText "You have turned off the electricity.")
        (Audio|PlaySoundatLocation "/Engine/VREditor/Sounds/UI/Dockable_Window_Close.Dockable_Window_Close" _returnvalue "0, 0, 0" 1.0 1.0 0.0 0 0 0 0)
        (Effects|SpawnEmitteratLocation "/Game/StarterContent/Particles/P_Smoke.P_Smoke" _returnvalue)))
    (else
      (Development|PrintText "You need a wrench to turn off the power!")
      (Audio|PlaySoundatLocation "/Engine/EditorSounds/Notifications/CompileFailed.CompileFailed" "0, 0, 0" "0, 0, 0" 1.0 1.0 0.0 0 0 0 0))))

(event EventTick
  (params (DeltaSeconds :type Float%20%28single-precision%29)))

(fn ConstructionScript)