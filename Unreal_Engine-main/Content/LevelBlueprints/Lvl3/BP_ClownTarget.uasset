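; BP_ClownTarget is a Level 3 clown target that gets knocked over by first-person projectiles.
; A projectile hit on the Box flags it knocked and enables Sphere physics with a zero impulse, then casts the hit actor to BP_GameManager.
; ResetClown restores physics, rotation and collision.
; The scoring, collision disabling and random reset timer are disconnected, so hits neither award points nor schedule a reset.
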(event OnComponentHit(Box)
  (params (HitComponent :type Primitive%20Component%20Object%20Reference) (OtherActor :type Actor%20Object%20Reference) (OtherComp :type Primitive%20Component%20Object%20Reference) (NormalImpulse :type Vector :default "0, 0, 0") (Hit :type Hit%20Result%20Structure%20%28by%20ref%29))
  (Utilities|Casting|CastToBP_FirstPersonProjectile OtherActor
    (:then
      (Variables|Default|SetisKnocked true)
      (Physics|SetSimulatePhysics (Variables|Default|GetSphere) true)
      (Physics|AddImpulse (Variables|Default|GetSphere) "0, 0, 0" "None" false)
      (bind _asbp_game_manager (Utilities|Casting|CastToBP_GameManager OtherActor)))
    (:CastFailed
      (Development|PrintText "Cast Failed"))))

(event Custom|ResetClown
  (if (Variables|Default|GetisKnocked)
    (Variables|Default|SetisKnocked false)
    (Physics|SetSimulatePhysics (Variables|Default|GetSphere) false)
    (Transformation|SetRelativeRotation (Variables|Default|GetSphere) "0, 0, 0" false false)
    (Collision|SetCollisionEnabled (Variables|Default|GetBox) "QueryAndPhysics")))

(event EventBeginPlay)

(event EventTick
  (params (DeltaSeconds :type Float%20%28single-precision%29)))

(fn ConstructionScript)